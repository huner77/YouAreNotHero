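; BP_Enemy is an enemy character that can be damaged by the player and flags when it is in melee range.
; Its trigger overlap registers or removes it in BP_Player's attacked-enemy array and toggles CanMelee.
; Attacked lowers HP, then either sets the death flag or clears IsAttacked after a delay.
; Helpers initialize stats and set walk speed; Stun is empty, and destroy and respawn logic is unwired.
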(event `self.Trriger.OnComponentBeginOverlap`
  (params (OverlappedComponent :type "PrimitiveComponent Object Reference") (OtherActor :type "Actor Object Reference") (OtherComp :type "PrimitiveComponent Object Reference") (OtherBodyIndex :type Integer) (bFromSweep :type Boolean) (SweepResult :type "HitResult Structure (by ref)"))
  (bind _asbp_player (cast `/Game/Character/BP_Player` OtherActor))
  (set `self.Ref_Player` _asbp_player)
  (`KismetArrayLibrary.Array_Add` (`/Game/Character/BP_Player.Array_AttackedEnemy` (`self.Ref_Player`)) self)
  (set `self.CanMelee` true))

(event `self.Trriger.OnComponentEndOverlap`
  (params (OverlappedComponent :type "PrimitiveComponent Object Reference") (OtherActor :type "Actor Object Reference") (OtherComp :type "PrimitiveComponent Object Reference") (OtherBodyIndex :type Integer))
  (cast `/Game/Character/BP_Player` OtherActor)
  (`KismetArrayLibrary.Array_RemoveItem` (`/Game/Character/BP_Player.Array_AttackedEnemy` (`self.Ref_Player`)) self)
  (set `self.CanMelee` false))

(event `Attacked`
  (params (AttackDamage :type Integer))
  (set `self.IsAttacked` true)
  (bind _output_get (set `self.CurrentHP` (- (`self.CurrentHP`) AttackDamage)))
  (if (<= _output_get 0)
    (`self.Death`)
    (else
      (`KismetSystemLibrary.Delay` 2.0)
      (set `self.IsAttacked` false))))

(event `Stun`
  (params (StunTime :type Integer)))

(fn `Death`
  (set `self.IsDeath` true))

(fn `InitInfo`
  (params (Level :type Integer) (EXP :type Integer) (HP :type Integer))
  (set `self.EXP` EXP)
  (set `self.Level` Level)
  (set `self.CurrentHP` HP))

(fn `UpdateWalkSpeed`
  (params (WalkSpeed :type "Float (double-precision)"))
  (set `CharacterMovementComponent.MaxWalkSpeed` WalkSpeed (`self.CharacterMovement`)))

(fn `UserConstructionScript`)