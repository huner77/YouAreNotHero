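; BP_B is a ranged character, apparently an enemy, that fires projectiles when the player is in range.
; The FireTrriger component's overlaps with BP_Player toggle CanFire and store a player reference.
; OnAttack, gated by CanFire and IsAttacked, spawns BP_Projectile at the actor's own transform and clears IsAttacking after a delay.
; The construction script sets its level, EXP and current HP.
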(event `self.ReceiveBeginPlay`
  (`parent.ReceiveBeginPlay`))

(event `self.FireTrriger.OnComponentBeginOverlap`
  (params (OverlappedComponent :type "PrimitiveComponent Object Reference") (OtherActor :type "Actor Object Reference") (OtherComp :type "PrimitiveComponent Object Reference") (OtherBodyIndex :type Integer) (bFromSweep :type Boolean) (SweepResult :type "HitResult Structure (by ref)"))
  (bind _asbp_player (cast `/Game/Character/BP_Player` OtherActor))
  (set `self.Ref_Player2` _asbp_player)
  (set `self.CanFire` true))

(event `self.FireTrriger.OnComponentEndOverlap`
  (params (OverlappedComponent :type "PrimitiveComponent Object Reference") (OtherActor :type "Actor Object Reference") (OtherComp :type "PrimitiveComponent Object Reference") (OtherBodyIndex :type Integer))
  (cast `/Game/Character/BP_Player` OtherActor)
  (set `self.CanFire` false))

(event `OnAttack`
  (if (and (`self.CanFire`) (not (`self.IsAttacked`)))
    (`self.Attacking`)
    (`KismetSystemLibrary.Delay` 2.0)
    (set `self.IsAttacking` false)))

(fn `Attacking`
  (set `self.IsAttacking` true)
  (`|SpawnActorFromClass` "/Game/Character/BP_Projectile.BP_Projectile_C" (`self.GetTransform` self) "Undefined" "MultiplyWithRoot" null null))

(fn `UserConstructionScript`
  (`parent.UserConstructionScript`)
  (set `self.Level` 5)
  (set `self.EXP` 3)
  (set `self.CurrentHP` 300))