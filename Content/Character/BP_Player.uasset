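; Player character with cancer-cell meshes, handling movement, pitch-limited look, jump, swept forward blink and HUD creation.
; Left click damages the first enemy in the attackable array; kills decrement per-type enemy counts and grant EXP, max HP and healing.
; Passing the EXP threshold raises the level and calls OnLevelUp, while UpdateSM provides per-level mesh swaps.
; HP is clamped and regenerates on a timer; H and G are cheat keys.
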(event `self.ReceiveTick`
  (params (DeltaSeconds :type "Float (single-precision)")))

(event `self.ReceiveBeginPlay`
  (`self.CreateHUD`)
  (`self.OnAddHPByTime`))

(event `InputAxis|MoveForward`
  (params (AxisValue :type "Float (single-precision)"))
  ;[1 1 1] 人物移动和视角移动
  (`self.AddMovementInput` (`KismetMathLibrary.GetForwardVector` (`KismetMathLibrary.MakeRotator` 0.0 0.0 (.yaw (`self.GetControlRotation`)))) AxisValue))

(event `InputAxis|MoveRight`
  (params (AxisValue :type "Float (single-precision)"))
  ;[1 1 1] 人物移动和视角移动
  (`self.AddMovementInput` (`KismetMathLibrary.GetRightVector` (`KismetMathLibrary.MakeRotator` 0.0 0.0 (.yaw (`self.GetControlRotation`)))) AxisValue))

(event `InputAxis|Turn`
  (params (AxisValue :type "Float (single-precision)"))
  ;[1 1 1] 人物移动和视角移动
  (`self.AddControllerYawInput` AxisValue))

(event `InputAxis|LookUp`
  (params (AxisValue :type "Float (single-precision)"))
  (bind _returnvalue (+ (* AxisValue (`PlayerController.GetDeprecatedInputPitchScale` (`GameplayStatics.GetPlayerController` 0))) (.pitch (`Controller.GetControlRotation` (`GameplayStatics.GetPlayerController` 0)))))
  ;[1 1 1] 人物移动和视角移动
  (if (or (and (> _returnvalue 300.0) (< _returnvalue 360.0)) (< _returnvalue 45.0))
    (`self.AddControllerPitchInput` AxisValue)))

(event `Key|SpaceBar`
  (params (Key :type "Key Structure"))
  ;[1 1 1] 人物技能
  (:`Pressed`
    (`self.Jump`))
  (:`Released`
    (`self.StopJumping`)))

(event `Key|LeftMouseButton`
  (params (Key :type "Key Structure"))
  ;[1 1 1] 人物技能
  (:`Pressed`
    (set `self.IsAttacking` true)
    (bind _newparam (`self.AttackOneEnemy`))
    (`/Engine/EditorBlueprintResources/StandardMacros.IsValid` _newparam
      (:`Is Valid`
        (`self.Attacking`))
      (:`Is Not Valid`
        _))
    (`KismetSystemLibrary.Delay` 1.0)
    (set `self.IsAttacking` false)))

(event `Key|LeftShift`
  (params (Key :type "Key Structure"))
  ;[1 1 1] 人物技能
  (:`Pressed`
    (`self.Blinking`)))

(event `Key|H`
  (params (Key :type "Key Structure"))
  ;[1 1 1] 金手指
  (:`Pressed`
    (set `self.CurrentHP` (- (`self.CurrentHP`) 10))))

(event `Key|G`
  (params (Key :type "Key Structure"))
  ;[1 1 1] 金手指
  (:`Pressed`
    (`self.LevelUp`)))

(event `OnAttacked`
  (params (DamageNum :type Integer))
  ;[1 1 1] 状态
  (bind _result (`/Engine/EditorBlueprintResources/StandardMacros.NegateInt` DamageNum)
    (:`  `
      (`self.UpdateCurrentHP` _result)
      (set `self.IsAttacked` true)
      (`KismetSystemLibrary.Delay` 0.5)
      (set `self.IsAttacked` false))))

(event `OnAddHPByTime`
  ;[1 1 1] 状态
  (`KismetSystemLibrary.K2_SetTimerDelegate` (delegate `OnAddHPByTime`) 1.0 true)
  (`self.UpdateCurrentHP` 1))

(fn `Attacking`
  (bind _attackedenemy (`self.AttackedEnemy`))
  (`/Game/Character/BP_Enemy.Attacked` _attackedenemy (`self.AttackDamage`))
  (if (`/Game/Character/BP_Enemy.IsDeath` _attackedenemy)
    (`self.UpdateEXP` _attackedenemy)
    (`self.DecreaseCurrentEnemy` _attackedenemy)
    (`self.K2_DestroyActor` _attackedenemy)
    (set `self.IsAttacking` false)))

(fn `AttackOneEnemy`
  (returns (NewParam :type "/Game/Character/BP_Enemy Object Reference"))
  (if (> (`KismetArrayLibrary.Array_Length` (`self.Array_AttackedEnemy`)) 0)
    (bind _output_get (set `self.AttackedEnemy` (`|GetArrayItem` (`self.Array_AttackedEnemy`))))
    (return _output_get)
    (else
      (return null))))

(fn `Blinking`
  (`self.K2_SetActorLocation` (+ (`self.K2_GetActorLocation`) (* (`self.GetActorForwardVector`) 300.0)) true))

(fn `CreateHUD`
  (bind _returnvalue (`|CreateWidget` "/Game/UI/UI_HUD.UI_HUD_C"))
  (bind _output_get (set `self.Ref_UIHUD` _returnvalue))
  (`UserWidget.AddToViewport` _output_get 0))

(fn `DecreaseCurrentEnemy`
  (params (Enemy :type "/Game/Character/BP_Enemy Object Reference"))
  (cast `/Game/Character/BP_B` Enemy
    (:`then`
      (set `self.CurrentEnemyBCount` (- (`self.CurrentEnemyBCount`) 1)))
    (:`CastFailed`
      (cast `/Game/Character/BP_Lymph` Enemy
        (:`then`
          (set `self.CurrentEnemyLymphCount` (- (`self.CurrentEnemyLymphCount`) 1)))
        (:`CastFailed`
          (cast `/Game/Character/BP_White` Enemy)
          (set `self.CurrentEnemyWhiteCount` (- (`self.CurrentEnemyWhiteCount`) 1)))))))

(fn `LevelUp`
  (set `self.CurrentEXP` 0)
  (set `self.CurrentLevel` (+ (`self.CurrentLevel`) 1))
  (`self.OnLevelUp`))

(fn `UpdateCurrentHP`
  (params (AddHP :type Integer))
  (bind _maxhp (`self.MaxHP`))
  (bind _returnvalue (+ (`self.CurrentHP`) AddHP))
  (if (< _returnvalue 0)
    (set `self.CurrentHP` 0)
    (elif (> _returnvalue _maxhp)
      (set `self.CurrentHP` _maxhp)
      (else
        (set `self.CurrentHP` _returnvalue)))))

(fn `UpdateEXP`
  (params (Enemy :type "/Game/Character/BP_Enemy Object Reference"))
  (bind _exp (`/Game/Character/BP_Enemy.EXP` Enemy))
  (set `self.CurrentEXP` (+ (`self.CurrentEXP`) _exp))
  (set `self.MaxHP` (+ _exp (`self.MaxHP`)))
  (`self.UpdateCurrentHP` _exp)
  (if (> (`self.CurrentEXP`) (`|GetArrayItem` (`self.LevelUpEXP`) (`self.CurrentLevel`)))
    (`self.LevelUp`)))

(fn `UpdateSM`
  (params (LevelIndex :type Integer))
  (bind _mesh (`self.Mesh`))
  (if (== LevelIndex 1)
    (`SkeletalMeshComponent.SetSkeletalMeshAsset` _mesh "/Game/donghua/zhujue_02/SM_Cancer_Lv2.SM_Cancer_Lv2")
    (elif (== LevelIndex 2)
      (`SkeletalMeshComponent.SetSkeletalMeshAsset` _mesh "/Game/donghua/zhujue_03/SM_CanCel_Lv3.SM_CanCel_Lv3"))))

(fn `UserConstructionScript`)