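; BP_Lymph is a character Blueprint, apparently an enemy, that damages the player when it attacks.
; On BeginPlay it runs the parent logic, then sets its own Level and EXP.
; Its Attacking function raises the IsAttacking flag and calls Attacked on the player reference, passing Damage.
; Overlap and Tick events are disabled, and the construction script only calls the parent.
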(event `self.ReceiveBeginPlay`
  (`parent.ReceiveBeginPlay`)
  (set `self.Level` 3)
  (set `self.EXP` 2))

(fn `Attacking`
  (set `self.IsAttacking` true)
  (`/Game/Character/BP_Player.Attacked` (`self.Ref_Player`) (`self.Damage`)))

(fn `UserConstructionScript`
  (`parent.UserConstructionScript`))